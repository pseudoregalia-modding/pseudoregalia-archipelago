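; In-world bridge actor for the AP randomizer mod, exposing AP functions that apply randomizer state to the game.
; Spawns and tracks collectible and interactable auras by ID, refreshing their visibility when options change.
; Writes upgrades, keys and health into MV_GameInstance, expanding progressive items, and also handles warps, popups, console and overlay widgets.
; Empty Tick lets C++ run game-thread actions; the remappable slide-jump toggle calls an empty stub.
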(event Input|EnhancedActionEvents|EnhancedInputActionIA_ToggleSlideJump
  (params (ActionValue :type Boolean) (ElapsedSeconds :type Float%20%28double-precision%29) (TriggeredSeconds :type Float%20%28double-precision%29) (InputAction :type Input%20Action%20Object%20Reference :default "/Game/Mods/AP_Randomizer/IA_ToggleSlideJump.IA_ToggleSlideJump"))
  (:Triggered
    (CallFunction|APToggleSlideJump)))

(event EventBeginPlay
  (Utilities|FlowControl|Sequence
    (:then_0
      (bind _returnvalue (Actor|GetActorOfClass "/Game/ThirdPerson/Player/BP_PlayerGoatMain.BP_PlayerGoatMain_C"))
      (Variables|Default|SetPlayerRef _returnvalue))
    (:then_1
      (bind _save (CallFunction|GetOptionsSave))
      (Variables|Default|SetOptions (Variables|/Game/Mods/AP_Randomizer/Options/BP_APOptionsSave.BP_APOptionsSave_C|GetOptions _save)))
    (:then_2
      (CallFunction|SetUpSolarWindToggle false))))

(event EventTick
  (params (DeltaSeconds :type Float%20%28single-precision%29))
  ;[1 1 1] empty eventtick used for running actions in the game thread from c++
)

(fn ConstructionScript)

(fn APSpawnCollectible
  (params (collectible_id :type Integer64) (collectible_position :type Vector) (PseudoType :type EPseudoType%20Enum :default "NewEnumerator0") (Classification :type EClassification%20Enum :default "NewEnumerator0"))
  (bind _options (Variables|Default|GetOptions))
  (bind (_pseudoitemdisplay _offworlditemdisplay) (Utilities|Struct|BreakF_APOptions _options))
  (bind _returnvalue (Game|SpawnActorfromClass "/Game/Mods/AP_Randomizer/BP_APCollectible.BP_APCollectible_C" (Math|Transform|MakeTransform (Math|Vector|MakeVector (.x collectible_position) (.y collectible_position) (+ (.z collectible_position) 1.5e+02)) "0, 0, 0" "1.000000,1.000000,1.000000") "Undefined" 0 collectible_id PseudoType Classification 0))
  (bind _output_get (LocalVariables|SetCollectible _returnvalue))
  (Default|SetVisibility _output_get _pseudoitemdisplay _offworlditemdisplay)
  (Utilities|Map|Add (Variables|Default|GetCollectibles) collectible_id (LocalVariables|GetCollectible)))

(fn APDespawnCollectible
  (params (id :type Integer64))
  (bind _collectibles (Variables|Default|GetCollectibles))
  (bind (_value _returnvalue) (Utilities|Map|Find _collectibles id))
  (if _returnvalue
    (Default|Despawn _value)
    (Utilities|Map|Remove (Variables|Default|GetCollectibles) id)))

(fn APSpawnInteractableAura
  (params (follow :type Object%20Object%20Reference) (interactableId :type Integer64) (classification :type EClassification%20Enum :default "NewEnumerator0"))
  (bind _asactor (Utilities|Casting|CastToActor follow))
  (bind _returnvalue (Game|SpawnActorfromClass "/Game/Mods/AP_Randomizer/BP_APInteractableAura.BP_APInteractableAura_C" (Math|Transform|MakeTransform (Transformation|GetActorLocation _asactor) "0, 0, 0" "1.000000,1.000000,1.000000") "Undefined" 0 _asactor interactableId classification 0))
  (bind _output_get (LocalVariables|SetInteractable _returnvalue))
  (Default|SetVisibility _output_get (.InteractableItemDisplay (Utilities|Struct|BreakF_APOptions (Variables|Default|GetOptions))))
  (Utilities|Map|Add (Variables|Default|GetInteractables) interactableId (LocalVariables|GetInteractable)))

(fn APDespawnInteractableAura
  (params (id :type Integer64))
  (bind _interactables (Variables|Default|GetInteractables))
  (bind (_value _returnvalue) (Utilities|Map|Find _interactables id))
  (if _returnvalue
    (Default|Despawn _value)
    (Utilities|Map|Remove (Variables|Default|GetInteractables) id)))

(fn APSetUpgrades
  (params (new_name :type Array%20of%20Names) (new_count :type Array%20of%20Integers) (disable_slidejump :type Boolean))
  (bind _asmv_game_instance (Utilities|Casting|CastToMV_GameInstance (Game|GetGameInstance)))
  (bind _output_get (LocalVariables|SetGameInstance _asmv_game_instance))
  (LocalVariables|Setnew_map (Variables|/Game/Blueprints/GameData/MV_GameInstance.MV_GameInstance_C|GetupgradeTracker _output_get))
  (Utilities|FlowControl|Sequence
    (:then_0
      ;[1 1 1] build upgrade map based on current map and params, take the max so the player can't lose upgrades
      (for (_array_element _array_index) new_name
        (Utilities|Map|Add (LocalVariables|Getnew_map) _array_element (Math|Integer|Max(Integer) (Utilities|Array|Get(acopy) new_count _array_index) (.Value (Utilities|Map|Find (LocalVariables|Getnew_map) _array_element))))))
    (:then_1
      ;[1 1 1] handle ~progressiveBreaker (default includes 3, the expected value for setting projectile; but also accounts for player using plando/!getitem)
      (switch int (.Value (Utilities|Map|Find (LocalVariables|Getnew_map) "~progressiveBreaker"))
        (:Default
          (Utilities|Map|Add (LocalVariables|Getnew_map) "projectile" 1)
          (Utilities|Map|Add (LocalVariables|Getnew_map) "chargeAttack" 1 :!label _label))
        (:1
          _)
        (:2
          (goto _label)))
      (Utilities|Map|Add (LocalVariables|Getnew_map) "attack" 1))
    (:then_2
      ;[1 1 1 1 16] handle ~progressiveSlide (default includes 2, the expected value for setting SlideJump; but also accounts for player using plando/!getitem)
      (switch int (.Value (Utilities|Map|Find (LocalVariables|Getnew_map) "~progressiveSlide"))
        (:Default
          (Utilities|Map|Add (LocalVariables|Getnew_map) "SlideJump" 1))
        (:1
          _))
      (Utilities|Map|Add (LocalVariables|Getnew_map) "slide" 1))
    (:then_3
      ;[1 1 1] handle ~solar
      (if (Math|Conversions|ToBoolean(Integer) (.Value (Utilities|Map|Find (LocalVariables|Getnew_map) "~solar")))
        (Utilities|Map|Add (LocalVariables|Getnew_map) "SlideJump" 1)))
    (:then_4
      ;[1 1 1] configure slide ui if slide + SlideJump (must do this before disabling SlideJump)
      (if (and (Math|Conversions|ToBoolean(Integer) (.Value (Utilities|Map|Find (LocalVariables|Getnew_map) "slide"))) (Math|Conversions|ToBoolean(Integer) (.Value (Utilities|Map|Find (LocalVariables|Getnew_map) "SlideJump"))))
        (CallFunction|ConfigureSlideUI disable_slidejump)))
    (:then_5
      ;[1 1 1] check for disabled slidejump
      (if disable_slidejump
        (Utilities|Map|Add (LocalVariables|Getnew_map) "SlideJump" 0)))
    (:then_6
      ;[1 1 1] handle ~cling#
      (if (or (Math|Conversions|ToBoolean(Integer) (.Value (Utilities|Map|Find (LocalVariables|Getnew_map) "~cling6"))) (Math|Conversions|ToBoolean(Integer) (.Value (Utilities|Map|Find (LocalVariables|Getnew_map) "~cling2"))))
        (Utilities|FlowControl|Sequence
          (:then_0
            (Utilities|Map|Add (LocalVariables|Getnew_map) "wallRide" 1))
          (:then_1
            (Variables|/Game/ThirdPerson/Player/BP_PlayerGoatMain.BP_PlayerGoatMain_C|SetwallRunClingLimit (Variables|Default|GetPlayerRef) (+ (* (Math|Integer|Clamp(Integer) (.Value (Utilities|Map|Find (LocalVariables|Getnew_map) "~cling6")) 0 1) 6) (* (.Value (Utilities|Map|Find (LocalVariables|Getnew_map) "~cling2")) 2) -1))))))
    (:then_7
      ;[1 1 1] clear out attack if value is 0 (to prevent fake breaker from disappearing
      (if (and (== (.Value (Utilities|Map|Find (LocalVariables|Getnew_map) "attack")) 0) (.ReturnValue (Utilities|Map|Find (LocalVariables|Getnew_map) "attack")))
        (Utilities|Map|Remove (LocalVariables|Getnew_map) "attack")))
    (:then_8
      ;[1 1 1] set upgrades in game instance and player
      (bind _output_get_2 (Variables|/Game/Blueprints/GameData/MV_GameInstance.MV_GameInstance_C|SetupgradeTracker (LocalVariables|GetGameInstance) (LocalVariables|Getnew_map)))
      (Default|UpdateUpgrades (Variables|Default|GetPlayerRef) _output_get_2))))

(fn APSetMajorKeys
  (params (keys :type Array%20of%20Booleans))
  (bind _asmv_game_instance (Utilities|Casting|CastToMV_GameInstance (Game|GetGameInstance)))
  (for (_array_element _array_index) keys
    (switch int _array_index
      (:0
        (Variables|/Game/Blueprints/GameData/MV_GameInstance.MV_GameInstance_C|Setkey1 _asmv_game_instance _array_element))
      (:1
        (Variables|/Game/Blueprints/GameData/MV_GameInstance.MV_GameInstance_C|Setkey2 _asmv_game_instance _array_element))
      (:2
        (Variables|/Game/Blueprints/GameData/MV_GameInstance.MV_GameInstance_C|Setkey3 _asmv_game_instance _array_element))
      (:3
        (Variables|/Game/Blueprints/GameData/MV_GameInstance.MV_GameInstance_C|Setkey4 _asmv_game_instance _array_element))
      (:4
        (Variables|/Game/Blueprints/GameData/MV_GameInstance.MV_GameInstance_C|Setkey5 _asmv_game_instance _array_element)))))

(fn APSetSmallKeys
  (params (key_count :type Integer))
  (bind _asmv_game_instance (Utilities|Casting|CastToMV_GameInstance (Game|GetGameInstance)))
  (Utilities|FlowControl|Sequence
    (:then_0
      ;[1 1 1] Count how many doors have been unlocked, and store the sum in spent_keys
      (for _array_element (Variables|/Game/Blueprints/GameData/MV_GameInstance.MV_GameInstance_C|GetallZoneDataStrs _asmv_game_instance)
        (bind _keys (Utilities|Map|Keys (.namesAndStates (Utilities|Struct|BreakST_ZoneData _array_element))))
        (for _array_element_2 _keys
          (if (Utilities|String|StartsWith _array_element_2 "BP_LockDoor")
            (LocalVariables|Setspent_keys (+ (LocalVariables|Getspent_keys) (.Value (Utilities|Map|Find (.namesAndStates (Utilities|Struct|BreakST_ZoneData _array_element)) _array_element_2))))))))
    (:then_1
      ;[1 1 1] Set NumberOfKeys to key_count - spent_keys.
      (bind _output_get (Variables|/Game/Blueprints/GameData/MV_GameInstance.MV_GameInstance_C|SetNumberOfKeys _asmv_game_instance (- key_count (LocalVariables|Getspent_keys))))
      (bind _foundwidgets (Widget|GetAllWidgetsOfClass "/Game/UI/UI_HUD.UI_HUD_C" true))
      (Default|UpdateKeyCountUI _foundwidgets _output_get))))

(fn APSetHealthPieces
  (params (healthpiece_count :type Integer))
  (bind _asmv_game_instance (Utilities|Casting|CastToMV_GameInstance (Game|GetGameInstance)))
  (if (> healthpiece_count (Variables|/Game/Blueprints/GameData/MV_GameInstance.MV_GameInstance_C|GethpPieces _asmv_game_instance))
    (Variables|/Game/Blueprints/GameData/MV_GameInstance.MV_GameInstance_C|SethpPieces _asmv_game_instance healthpiece_count)
    (Default|HealPlayer (Variables|Default|GetPlayerRef) 1e+02)))

(fn APToggleSlideJump
  (return))

(fn ConfigureSlideUI
  (params (slide :type Boolean))
  ;[1 1 1] don't add widget to a non gameplay level
  (bind _returnvalue (Game|GetCurrentLevelName true))
  (if (not (or (Utilities|Enum|Equal(Enum) _returnvalue "TitleScreen") (Utilities|Enum|Equal(Enum) _returnvalue "EndScreen")))
    (Utilities|FlowControl|Sequence
      (:then_0
        (Utilities|IsValid (Variables|Default|GetSlideIconRef)
          (:Is%20Not%20Valid
            (bind _returnvalue_2 (UserInterface|CreateWidget "/Game/Mods/AP_Randomizer/AP_SlideIcon.AP_SlideIcon_C"))
            (bind _output_get (Variables|Default|SetSlideIconRef _returnvalue_2))
            (UserInterface|Viewport|AddtoViewport _output_get -1))))
      (:then_1
        (Default|SetIcon (Variables|Default|GetSlideIconRef) slide)))))

(fn APPrintItemMessage
  (params (preamble :type Text) (item :type Text) (location :type Text) (mute_sound :type Boolean))
  (bind _returnvalue (UserInterface|CreateWidget "/Game/Mods/AP_Randomizer/WBP_ItemMiniPopup.WBP_ItemMiniPopup_C" (Game|GetPlayerController 0) preamble item location))
  (UserInterface|Viewport|AddtoViewport _returnvalue 0)
  (if (not mute_sound)
    (Audio|PlaySound2D "/Game/Audio/Sounds/cue_keyGet.cue_keyGet" 0.8 1.0 0.0 0 0)))

(fn APWarp
  (params (zone :type String) (playerStart :type String))
  (bind _asmv_game_instance (Utilities|Casting|CastToMV_GameInstance (Game|GetGameInstance)))
  (Default|UpdateZoneandSavePoint _asmv_game_instance zone "" playerStart)
  (Default|ReloadandRespawn _asmv_game_instance))

(fn APAddMessages
  (params (markdown_messages :type Array%20of%20Texts) (plain_messages :type Array%20of%20Texts) (show_console :type Boolean))
  (Default|APAddMessages (Variables|Default|Getconsole_ref) markdown_messages plain_messages show_console))

(fn APCreateConsole
  (bind _returnvalue (Game|GetCurrentLevelName true))
  (if (Variables|Default|Getconsole_exists)
    (Variables|Default|Setconsole_exists false) ; This function is typically called in response the the HUD being created because we want the\nconsole to be on top of the HUD. After the great door cutscene plays, it recreates the HUD,\nso we need a way to refresh the console.
    (Variables|Default|Setconsole_initialized false)
    (Widget|RemovefromParent (Variables|Default|Getconsole_ref)))
  (bind _returnvalue_2 (UserInterface|CreateWidget "/Game/Mods/AP_Randomizer/AP_DeluxeConsole.AP_DeluxeConsole_C" (Game|GetPlayerController 0)))
  (bind _output_get (Variables|Default|Setconsole_ref _returnvalue_2))
  (UserInterface|Viewport|AddtoViewport _output_get (Math|Integer|SelectInt 1 0 (Utilities|Enum|Equal(Enum) _returnvalue "EndScreen")))
  (Variables|Default|Setconsole_exists true))

(fn APPrintMessage
  (params (message :type Text) (mute_sound :type Boolean))
  (bind _returnvalue (UserInterface|CreateWidget "/Game/Mods/AP_Randomizer/WBP_MiniPopup.WBP_MiniPopup_C" (Game|GetPlayerController 0) message))
  (UserInterface|Viewport|AddtoViewport _returnvalue 0)
  (if (not mute_sound)
    (Audio|PlaySound2D "/Game/Audio/Sounds/cue_keyGet.cue_keyGet" 0.8 1.0 0.0 0 0)))

(fn APMarkGameCompleted
  (bind _asmv_game_instance (Utilities|Casting|CastToMV_GameInstance (Game|GetGameInstance)))
  (CallFunction|SetGameCompleted (Variables|/Game/Blueprints/GameData/MV_GameInstance.MV_GameInstance_C|GetactiveSaveSlotName _asmv_game_instance)))

(fn APCreateOverlay
  (params (Version :type Text))
  (bind _returnvalue (UserInterface|CreateWidget "/Game/Mods/AP_Randomizer/AP_VersionOverlay.AP_VersionOverlay_C" (Game|GetPlayerController 0) Version))
  (UserInterface|Viewport|AddtoViewport _returnvalue -2))

(fn APCreateConsoleHacky
  (bind _returnvalue (Game|GetPlayerController 0))
  ;[1 1 1] This is called when loading the title screen. For some reason this fixes an issue with the map. I don't know why. (kill me)
  (bind _returnvalue_2 (UserInterface|CreateWidget "/Game/Mods/AP_Randomizer/AP_DeluxeConsole.AP_DeluxeConsole_C" _returnvalue))
  (UserInterface|Viewport|AddtoViewport _returnvalue_2 0)
  (bind _returnvalue_3 (UserInterface|CreateWidget "/Game/Mods/AP_Randomizer/AP_DeluxeConsole.AP_DeluxeConsole_C" _returnvalue))
  (UserInterface|Viewport|AddtoViewport _returnvalue_3 0))

(fn UpdateOptions
  (params (NewOptions :type F%20AP%20Options%20Structure))
  (bind (_pseudoitemdisplay _offworlditemdisplay _interactableitemdisplay) (Utilities|Struct|BreakF_APOptions NewOptions))
  (LocalVariables|SetUpdateCollectibles (or (Utilities|Enum|NotEqual(Enum) _pseudoitemdisplay (.PseudoItemDisplay (Utilities|Struct|BreakF_APOptions (Variables|Default|GetOptions)))) (Utilities|Enum|NotEqual(Enum) _offworlditemdisplay (.OffWorldItemDisplay (Utilities|Struct|BreakF_APOptions (Variables|Default|GetOptions))))))
  (LocalVariables|SetUpdateInteractables (Utilities|Enum|NotEqual(Enum) _interactableitemdisplay (.InteractableItemDisplay (Utilities|Struct|BreakF_APOptions (Variables|Default|GetOptions)))))
  (bind _output_get (Variables|Default|SetOptions NewOptions))
  (Utilities|FlowControl|Sequence
    (:then_0
      (CallFunction|SetUpSolarWindToggle true))
    (:then_1
      (if (LocalVariables|GetUpdateCollectibles)
        (bind _values (Utilities|Map|Values (Variables|Default|GetCollectibles)))
        (for _array_element _values
          (Default|SetVisibility _array_element (.PseudoItemDisplay (Utilities|Struct|BreakF_APOptions _output_get)) (.OffWorldItemDisplay (Utilities|Struct|BreakF_APOptions _output_get))))))
    (:then_2
      (if (LocalVariables|GetUpdateInteractables)
        (bind _values_2 (Utilities|Map|Values (Variables|Default|GetInteractables)))
        (for _array_element_2 _values_2
          (Default|SetVisibility _array_element_2 (.InteractableItemDisplay (Utilities|Struct|BreakF_APOptions _output_get))))))))

(fn SetUpSolarWindToggle
  (params (Reset :type Boolean))
  (bind _returnvalue (Game|GetPlayerController 0))
  (bind _inputmappingcontext (Variables|Default|GetInputMappingContext))
  (bind _options (Variables|Default|GetOptions))
  (bind (_swtogglekey _swtogglepad) (Utilities|Struct|BreakF_APOptions _options))
  (bind _returnvalue_2 (PlayerController|LocalPlayerSubsystems|GetEnhancedInputLocalPlayerSubsystem _returnvalue))
  (Class|InputMappingContext|UnmapAllKeysfromAction _inputmappingcontext "/Game/Mods/AP_Randomizer/IA_ToggleSlideJump.IA_ToggleSlideJump")
  (Class|InputMappingContext|MapKey _inputmappingcontext "/Game/Mods/AP_Randomizer/IA_ToggleSlideJump.IA_ToggleSlideJump" _swtogglekey)
  (Class|InputMappingContext|MapKey _inputmappingcontext "/Game/Mods/AP_Randomizer/IA_ToggleSlideJump.IA_ToggleSlideJump" _swtogglepad)
  (if Reset
    (Input|RemoveMappingContext _returnvalue_2 _inputmappingcontext "(bIgnoreAllPressedKeysUntilRelease=True,bForceImmediately=False)"))
  (Input|AddMappingContext _returnvalue_2 _inputmappingcontext 0 "(bIgnoreAllPressedKeysUntilRelease=True,bForceImmediately=False)"))