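; BP_APInteractableAura is a Niagara aura actor for the Archipelago randomizer mod that visually marks an interactable.
; Each tick it moves itself to its Follow actor's location.
; SetVisibility resets the aura, then assigns a gold, green or pink effect by item classification, with a camera ring effect for Unknown or Basic display.
; Despawn hides the actor rather than destroying it.
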(event EventTick
  (params (DeltaSeconds :type Float%20%28single-precision%29))
  (Transformation|SetActorLocation (Transformation|GetActorLocation (Variables|Default|Getfollow)) false false))

(fn ConstructionScript)

(fn Despawn
  (Rendering|SetActorHiddenInGame true))

(fn SetVisibility
  (params (InteractableDisplay :type EInteractableDisplay%20Enum :default "NewEnumerator0"))
  (CallFunction|ResetAura)
  (switch Utilities|FlowControl|Switch|SwitchonEInteractableDisplay InteractableDisplay
    (:NewEnumerator0
      (switch Utilities|FlowControl|Switch|SwitchonEClassification (Variables|Default|GetClassification)
        (:NewEnumerator0
          (CallFunction|SetAura "/Game/VFX/Systems/NS_GoldAura.NS_GoldAura"))
        (:NewEnumerator1
          (CallFunction|SetAura "/Game/Mods/CustomVFX/NS_GreenAura.NS_GreenAura"))
        (:NewEnumerator2
          (CallFunction|SetAura "/Game/VFX/Systems/NS_PinkAura.NS_PinkAura"))
        (:NewEnumerator3
          (CallFunction|SetAura "/Game/VFX/Systems/NS_CameraRingAuraSave.NS_CameraRingAuraSave" :!label _label))))
    (:NewEnumerator1
      (goto _label))))

(fn SetAura
  (params (niagara :type Niagara%20System%20Object%20Reference))
  (bind _aura (Variables|Default|GetAura))
  (Class|NiagaraComponent|SetAsset _aura niagara true)
  (Rendering|SetVisibility _aura true true))

(fn ResetAura
  (Rendering|SetVisibility (Variables|Default|GetAura) false true))